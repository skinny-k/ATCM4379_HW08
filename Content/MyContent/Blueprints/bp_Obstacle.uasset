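; An obstacle actor that spins around its roll axis and knocks the third-person player character into ragdoll on contact.
; BeginPlay gives it a random starting roll, and Tick keeps rolling it by RotationSpeed scaled by delta seconds.
; A capsule overlap casts the other actor to BP_ThirdPersonCharacter and calls its Ragdoll function.
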(event OnComponentBeginOverlap(Capsule)
  (params (OverlappedComponent :type Primitive%20Component%20Object%20Reference) (OtherActor :type Actor%20Object%20Reference) (OtherComp :type Primitive%20Component%20Object%20Reference) (OtherBodyIndex :type Integer) (bFromSweep :type Boolean) (SweepResult :type Hit%20Result%20Structure%20%28by%20ref%29))
  (bind _asbp_third_person_character (Utilities|Casting|CastToBP_ThirdPersonCharacter OtherActor))
  (Default|Ragdoll _asbp_third_person_character))

(event EventBeginPlay
  (Transformation|AddActorLocalRotation (Math|Rotator|MakeRotator (Math|Random|RandomFloatinRange 0.0 1.8e+02) 0.0 0.0) false false))

(event Collision|EventActorBeginOverlap
  (params (OtherActor :type Actor%20Object%20Reference)))

(event EventTick
  (params (DeltaSeconds :type Float%20%28single-precision%29))
  (Transformation|AddActorLocalRotation (Math|Rotator|MakeRotator (* DeltaSeconds (Variables|Default|GetRotation%20Speed)) 0.0 0.0) false false))

(fn ConstructionScript)